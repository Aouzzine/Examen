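; UIBomb is an actor that spawns a Bomb at the world point under the mouse cursor when its Widget component is clicked.
; The click sets Game and UI input mode and creates and stores a SpawnBomb widget, which this graph never adds to the screen.
; A complex visibility trace under the cursor supplies the Bomb's spawn location, which is also printed for debugging.
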(event OnClicked(Widget)
  (params (TouchedComponent :type Primitive%20Component%20Object%20Reference))
  (bind _returnvalue (Game|GetPlayerController 0))
  (bind _hitresult (Game|Player|GetHitResultUnderCursorbyChannel _returnvalue "TraceTypeQuery1" true))
  (bind _location (Collision|BreakHitResult _hitresult))
  (bind (_x _y _z) (Math|Vector|BreakVector _location))
  (Input|SetInputModeGameandUI _returnvalue 0 false false)
  (bind _returnvalue_2 (UserInterface|CreateWidget "/Game/Blueprints/Bomb/SpawnBomb.SpawnBomb_C"))
  (Variables|Default|SetNewVar0 _returnvalue_2)
  (Game|SpawnActorfromClass "/Game/Blueprints/Bomb/Bomb.Bomb_C" (Math|Conversions|ToTransform(Vector) (Math|Vector|MakeVector _x _y _z)) false 0)
  (Development|PrintString "Spawned")
  (Development|PrintString (Utilities|String|ToString(Vector) _location)))

(event EventActorBeginOverlap
  (params (OtherActor :type Actor%20Object%20Reference)))

(event EventTick
  (params (DeltaSeconds :type Float%20%28single-precision%29)))

(fn ConstructionScript)